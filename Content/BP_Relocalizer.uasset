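; AR relocalizer that realigns tracking whenever a new fiducial image is detected and matched to an FAnchor in the scene.
; Each Tick during a running AR session, it prunes lost fiducials and matches new images to FAnchors by actor tag equal to image name.
; A detection sets the alignment to the inverse image tracking transform, unpins any previous pin and announces the anchor.
; The PinComponent call for the pawn root is disconnected.
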(event EventBeginPlay)

(event EventTick
  (params (DeltaSeconds :type Float%20%28single-precision%29))
  ;[1 0.3677 0.3711] Track Fiducials
  (switch Utilities|FlowControl|Switch|SwitchonEARSessionStatus (.Status (Utilities|Struct|BreakARSessionStatus (Class|ARBlueprintLibrary|GetARSessionStatus)))
    (:Running
      (bind _returnvalue (Class|ARBlueprintLibrary|GetAllTrackedImages))
      (CallFunction|CheckActiveFiducials _returnvalue)
      (for _array_element _returnvalue
        (if (not (== (Math|Transform|MakeTransform "0, 0, 0") (Class|ARTrackedGeometry|GetLocaltoTrackingTransform _array_element)))
          (if (not (Utilities|Map|Contains (Variables|Default|GettrackedFiducials) (Class|ARCandidateImage|GetFriendlyName (Class|ARTrackedImage|GetDetectedImage _array_element))))
            (bind _outactors (Actor|GetAllActorswithTag (Utilities|String|StringToName (Class|ARCandidateImage|GetFriendlyName (Class|ARTrackedImage|GetDetectedImage _array_element)))))
            (switch int (Utilities|Array|Length _outactors)
              (:Default
                (Class|DDBlueprintLibrary|LogWarning (Utilities|String|ToString(Text) (Utilities|Text|FormatText "Fiducial {imageName} has more than one fanchor. Will use the first one." (Utilities|Text|ToText(String) (Class|ARCandidateImage|GetFriendlyName (Class|ARTrackedImage|GetDetectedImage _array_element))))))
                (Utilities|Map|Add (Variables|Default|GettrackedFiducials) (Class|ARCandidateImage|GetFriendlyName (Class|ARTrackedImage|GetDetectedImage _array_element)) _array_element :!label _label)
                (bind _asfanchor (Utilities|Casting|CastToFAnchor (Utilities|Array|Get(acopy) _outactors)))
                (CallFunction|NewFiducialDetected _array_element _asfanchor))
              (:0
                (Class|DDBlueprintLibrary|LogWarning (Utilities|String|ToString(Text) (Utilities|Text|FormatText "Fiducial {imageName} but no corresponding fanchor was found in the scene." (Utilities|Text|ToText(String) (Class|ARCandidateImage|GetFriendlyName (Class|ARTrackedImage|GetDetectedImage _array_element)))))))
              (:1
                (Class|DDBlueprintLibrary|LogDebug (Utilities|String|ToString(Text) (Utilities|Text|FormatText "Detected fiducial {imageName}" (Utilities|Text|ToText(String) (Class|ARCandidateImage|GetFriendlyName (Class|ARTrackedImage|GetDetectedImage _array_element))))))
                (goto _label)))))))))

(fn NewFiducialDetected
  (params (arImage :type AR%20Tracked%20Image%20Object%20Reference) (fanchor :type F%20Anchor%20Object%20Reference))
  (bind _returnvalue (Class|ARTrackedGeometry|GetLocaltoTrackingTransform arImage))
  (Utilities|FlowControl|Sequence
    (:then_0
      (Variables|Default|SetanchorLocalTransform _returnvalue)
      (Variables|Default|SetanchorWorldTransform (Class|ARTrackedGeometry|GetLocaltoWorldTransform arImage))
      (Class|DDBlueprintLibrary|LogDebug "Set AR Alignment")
      (Class|ARBlueprintLibrary|SetAlignmentTransform (Math|Transform|InvertTransform _returnvalue)))
    (:then_1
      (if (Utilities|IsValid (Variables|Default|GetlastFanchor))
        (Class|ARBlueprintLibrary|UnpinComponent (Variables|/Script/Engine.Actor|GetRootComponent (Pawn|GetControlledPawn (Game|GetPlayerController 0)))))
      (Variables|Default|SetlastFanchor (stale _returnvalue))
      (Default|CallOnNewFiducialAnchored (Class|ARCandidateImage|GetFriendlyName (Class|ARTrackedImage|GetDetectedImage arImage)) (Transformation|GetActorTransform fanchor) fanchor))))

(fn CheckActiveFiducials
  (params (trackedImages :type Array%20of%20AR%20Tracked%20Image%20Object%20References))
  (bind _keys (Utilities|Map|Keys (Variables|Default|GettrackedFiducials)))
  (LocalVariables|SetforRemoval _keys)
  (for _array_element trackedImages
    (if (Utilities|Map|Contains (Variables|Default|GettrackedFiducials) (Class|ARCandidateImage|GetFriendlyName (Class|ARTrackedImage|GetDetectedImage _array_element)))
      (Utilities|Array|RemoveItem (LocalVariables|GetforRemoval) (Class|ARCandidateImage|GetFriendlyName (Class|ARTrackedImage|GetDetectedImage _array_element)))))
  (for _array_element_2 (LocalVariables|GetforRemoval)
    (Utilities|Map|Remove (Variables|Default|GettrackedFiducials) _array_element_2)
    (Class|DDBlueprintLibrary|LogDebug (Utilities|String|ToString(Text) (Utilities|Text|FormatText "Fiducial {imageName} not tracked anymore" (Utilities|Text|ToText(String) _array_element_2))))))