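; BP_Fanchor is a fiducial anchor actor that displays an AR candidate image on a plane, labeled with its name and streaming levels.
; On BeginPlay it takes its fiducial name from the candidate image, warning on mismatch, then textures a dynamic material and scales the plane by the image's width-to-height ratio.
; Tick turns both labels using the player controller's rotation.
; SetMaterialParams exposes the material's UV parameters.
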(event EventBeginPlay
  (bind _candidateimage (Variables|Default|GetcandidateImage))
  (bind _returnvalue (Class|ARCandidateImage|GetPhysicalHeight _candidateimage))
  (bind _returnvalue_2 (Class|ARCandidateImage|GetPhysicalWidth _candidateimage))
  (bind _returnvalue_3 (/ _returnvalue_2 _returnvalue))
  (CallFunction|OverrideFiducialName)
  (CallFunction|SetupLabels)
  ;[1 1 1] setup plane material with the candidate image texture
  (Utilities|IsValid (Variables|Default|GetcandidateImage)
    (:Is%20Valid
      (bind _returnvalue_4 (Rendering|Material|CreateDynamicMaterialInstance (Variables|Default|GetPlane) 0 "/FiducialRelocalizer/Materials/M_FiducialImageMaterial.M_FiducialImageMaterial" "None" :!class /Script/Engine.PrimitiveComponent))
      (bind _output_get (Variables|Default|SetimageMaterial _returnvalue_4))
      (Rendering|Material|SetTextureParameterValue _output_get "Texture" (Class|ARCandidateImage|GetCandidateTexture (Variables|Default|GetcandidateImage)))
      (if (> _returnvalue_3 1.0)
        (Transformation|SetRelativeScale3D (Variables|Default|GetPlane) (Math|Vector|MakeVector _returnvalue_3 1.0 1.0))
        (else
          (Transformation|SetRelativeScale3D (Variables|Default|GetPlane) (Math|Vector|MakeVector 1.0 _returnvalue_3 1.0)))))))

(event Collision|EventActorBeginOverlap
  (params (OtherActor :type Actor%20Object%20Reference)))

(event EventTick
  (params (DeltaSeconds :type Float%20%28single-precision%29))
  ;[1 1 1] face player always
  (CallFunction|SetFacePlayerCamera (Variables|Default|Getname))
  (CallFunction|SetFacePlayerCamera (Variables|Default|Getlevels)))

(fn ConstructionScript)

(fn SetupLabels
  (Rendering|Components|TextRender|SetText (Variables|Default|Getname) (Utilities|Text|FormatText "{aname} / {fname}" (Utilities|GetDisplayName self) (Variables|Default|GetFiducialName)))
  (Rendering|Components|TextRender|SetText (Variables|Default|Getlevels) (Utilities|Text|ToText(String) (CallFunction|NameArraytoString (Variables|Default|GetStreamingLevels) "
"))))

(fn SetFacePlayerCamera
  (params (component :type Scene%20Component%20Object%20Reference))
  (Transformation|SetWorldRotation component (.Rotation (Math|Transform|BreakTransform (Transformation|GetActorTransform (Game|GetPlayerController 0)))) false false)
  (Transformation|AddLocalRotation component "0,180.000000, 0" false false))

(fn SetMaterialParams
  (params (u1 :type Float%20%28single-precision%29) (v1 :type Float%20%28single-precision%29) (u2 :type Float%20%28single-precision%29) (v2 :type Float%20%28single-precision%29))
  (bind _imagematerial (Variables|Default|GetimageMaterial))
  (Rendering|Material|SetScalarParameterValue _imagematerial "u1" u1 :!class /Script/Engine.MaterialInstanceDynamic)
  (Rendering|Material|SetScalarParameterValue _imagematerial "v1" v1 :!class /Script/Engine.MaterialInstanceDynamic)
  (Rendering|Material|SetScalarParameterValue _imagematerial "u2" u2 :!class /Script/Engine.MaterialInstanceDynamic)
  (Rendering|Material|SetScalarParameterValue _imagematerial "v2" v2 :!class /Script/Engine.MaterialInstanceDynamic))

(fn OverrideFiducialName
  (bind _candidateimage (Variables|Default|GetcandidateImage))
  (bind _returnvalue (Class|ARCandidateImage|GetFriendlyName _candidateimage))
  (Utilities|IsValid _candidateimage
    (:Is%20Valid
      (if (and (not (Utilities|Array|IsEmpty (Variables|Default|GetFiducialName))) (Utilities|Enum|NotEqual(Enum) (Variables|Default|GetFiducialName) _returnvalue))
        (Class|DDBlueprintLibrary|LogWarning (Utilities|String|ToString(Text) (Utilities|Text|FormatText "Fiducial {fname} has name {n} but connected to candidate image {img}. Will override with candidate image name." (Utilities|GetDisplayName self) (Variables|Default|GetFiducialName) _returnvalue))))
      (Variables|Default|SetFiducialName _returnvalue))))